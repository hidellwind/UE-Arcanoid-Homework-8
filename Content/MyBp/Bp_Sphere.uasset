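; Bp_Sphere is a physics ball that launches along the player pawn's forward vector at BeginPlay and gains speed with every hit.
; Each hit adds an impulse along the hit normal scaled by Speed, offset in X and Y by the gained speed when either component is near zero.
; Spheres copy the pawn's count, decrement each other's on destruction, and end the game and destroy the pawn at zero.
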(event `self.ReceiveBeginPlay`
  (set `self.Speed` (`self.InitialSpeed`))
  (bind _output_get (set `self.PlayerActor` (cast `/Game/ThirdPerson/Blueprints/Bp_MyMainPawn` (`GameplayStatics.GetPlayerPawn` 0) :!pure true)))
  (set `self.CountSpheres` (`/Game/ThirdPerson/Blueprints/Bp_MyMainPawn.Count Spheres` _output_get))
  (`PrimitiveComponent.SetPhysicsLinearVelocity` (`self.Sphere`) (* (`self.GetActorForwardVector` (`self.PlayerActor`)) (`self.Speed`)) false "None")
  (bind _asbp_game_mode (cast `/Game/MyBp/Bp_GameMode` (`GameplayStatics.GetGameMode`)))
  (set `self.GameMode` _asbp_game_mode)
  (add `/Game/ThirdPerson/Blueprints/Bp_MyMainPawn.incrementCountSpheres` (`self.PlayerActor`) (delegate `addCountSphere`)))

(event `addCountSphere`
  (params (CountSpheres :type Integer))
  (set `self.CountSpheres` CountSpheres))

(event `self.Sphere.OnComponentHit`
  (params (HitComponent :type "PrimitiveComponent Object Reference") (OtherActor :type "Actor Object Reference") (OtherComp :type "PrimitiveComponent Object Reference") (NormalImpulse :type "Vector Structure") (Hit :type "HitResult Structure (by ref)"))
  (set `self.Speed` (+ (`self.Speed`) 5.0))
  (`self.Bounce` NormalImpulse))

(event `self.ReceiveDestroyed`
  (bind _outactors (`GameplayStatics.GetAllActorsOfClass` "Bp_Sphere_C"))
  (for _array_element _outactors
    (`self.decrementSpheres` _array_element))
  (if (== (`self.CountSpheres`) 0)
    (`/Game/MyBp/Bp_GameMode.EndGame` (`self.GameMode`))
    (`self.K2_DestroyActor` (`self.PlayerActor`))))

(event `decrementSpheres`
  (`/Engine/EditorBlueprintResources/StandardMacros.DecrementInt` (`self.CountSpheres`)))

(fn `Bounce`
  (params (NormalImpulse :type "Vector Structure"))
  (locals (ImpulseVector :type "Vector Structure"))
  (bind (_impulsevector_x _impulsevector_y) (`KismetMathLibrary.BreakVector` (`local.ImpulseVector`)))
  (bind (_x _y) (`KismetMathLibrary.BreakVector3f` (`local.ImpulseVector`)))
  (bind _returnvalue (- (`self.Speed`) (`self.InitialSpeed`)))
  (set `local.ImpulseVector` (* (`KismetMathLibrary.Normal` NormalImpulse) (`self.Speed`)))
  (if (or (and (>= _x -1.0) (<= _x 1.0)) (and (>= _y -1.0) (<= _y 1.0)))
    (bind _output_get (set `local.ImpulseVector` (`KismetMathLibrary.MakeVector` (+ _impulsevector_x _returnvalue) (+ _impulsevector_y _returnvalue)))))
  (`PrimitiveComponent.AddImpulse` (`self.Sphere`) _output_get "None" false))

(fn `PointAtTheCharacter`
  (locals (PlayerLocation :type "Vector Structure") (StoneLocation :type "Vector Structure") (MoveDirection :type "Vector Structure") (LaunchVelocity :type "Vector Structure")))

(fn `UserConstructionScript`)