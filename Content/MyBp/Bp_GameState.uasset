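; Game state Blueprint that tracks play time, a block count and whether the game has ended.
; BeginPlay enables Tick and caches the game mode; Tick adds delta time to TimePlayed but truncates each sum, dropping fractional seconds.
; AddBlock increments MaxCountBlock.
; The endgame event stops Tick, flags the game ended and passes the first player state's score to the game instance's high-score update.
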(event `self.ReceiveBeginPlay`
  (`self.SetActorTickEnabled` true)
  (set `self.GameMode` (cast `/Game/MyBp/Bp_GameMode` (`GameplayStatics.GetGameMode`) :!pure true))
  (set `self.IsGameEnded` false))

(event `self.ReceiveTick`
  (params (DeltaSeconds :type "Float (single-precision)"))
  (set `self.TimePlayed` (`KismetMathLibrary.FTrunc` (+ DeltaSeconds (`self.TimePlayed`)))))

(event `end game`
  (`self.SetActorTickEnabled` false)
  (set `self.IsGameEnded` true)
  (`/Game/MyBp/Bp_GameInstance.UpdateHighestScore` (cast `/Game/MyBp/Bp_GameInstance` (`GameplayStatics.GetGameInstance`) :!pure true) (`/Game/MyBp/Bp_PlayerState.PlayerScore` (cast `/Game/MyBp/Bp_PlayerState` (`GameplayStatics.GetPlayerState` 0) :!pure true))))

(fn `addBlock`
  (`/Engine/EditorBlueprintResources/StandardMacros.IncrementInt` (`self.maxCountBlock`)))

(fn `UserConstructionScript`)