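; Game mode Blueprint that handles ending and restarting a match.
; On BeginPlay it caches the game state as Bp_GameState, which holds the game-ended flag.
; EndGame forwards to the game state, and Restart_Game reloads the current level by name only once the game has ended.
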(event `self.ReceiveBeginPlay`
  (set `self.Game_State` (cast `/Game/MyBp/Bp_GameState` (`GameplayStatics.GetGameState`) :!pure true)))

(event `Restart_Game`
  (if (`/Game/MyBp/Bp_GameState.IsGameEnded` (`self.Game_State`))
    (bind _returnvalue (`GameplayStatics.GetCurrentLevelName` true))
    (`GameplayStatics.OpenLevel` (`KismetStringLibrary.Conv_StringToName` _returnvalue))))

(event `EndGame`
  (`/Game/MyBp/Bp_GameState.end game` (`self.Game_State`)))

(fn `UserConstructionScript`)