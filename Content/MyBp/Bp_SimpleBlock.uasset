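; Brick-breaker block that loses a life per hit, changes glow color, and destroys itself at zero.
; Construction script randomizes type and life (near-infinite for indestructible), coloring a dynamic material to match, with only some rolls yielding special types.
; It registers with Bp_GameState on BeginPlay.
; On destruction it ends the game if the block count is below one, otherwise awards MaxLife as score and triggers its type's player effect.
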(event `self.ReceiveBeginPlay`
  (set `self.CountLife` (`self.MaxLife`))
  (bind _asbp_game_state (cast `/Game/MyBp/Bp_GameState` (`GameplayStatics.GetGameState`)))
  (bind _output_get (set `self.GameState` _asbp_game_state))
  (`/Game/MyBp/Bp_GameState.addBlock` _output_get))

(event `self.Cube.OnComponentHit`
  (params (HitComponent :type "PrimitiveComponent Object Reference") (OtherActor :type "Actor Object Reference") (OtherComp :type "PrimitiveComponent Object Reference") (NormalImpulse :type "Vector Structure") (Hit :type "HitResult Structure (by ref)"))
  (bind _countlife (`self.CountLife`))
  (`/Engine/EditorBlueprintResources/StandardMacros.DecrementInt` _countlife
    (:`  `
      (`self.ChangeColor`)
      (if (== _countlife 0)
        (`self.K2_DestroyActor` self)))))

(event `self.ReceiveDestroyed`
  (if (< (`/Game/MyBp/Bp_GameState.maxCountBlock` (`self.GameState`)) 1)
    (`/Game/MyBp/Bp_GameState.end game` (`self.GameState`))
    (else
      (bind _asbp_player_state (cast `/Game/MyBp/Bp_PlayerState` (`GameplayStatics.GetPlayerState` 0)))
      (`/Game/MyBp/Bp_PlayerState.AddPlayerScore` _asbp_player_state (`self.MaxLife`))
      (bind _asbp_my_main_pawn (cast `` (`GameplayStatics.GetPlayerPawn` 0)))
      (`self.ChangesByBlockType` _asbp_my_main_pawn (`self.BlockType`)))))

(fn `ChangeColor`
  (switch `int` (`self.CountLife`)
    (:`1`
      (`MaterialInstanceDynamic.SetVectorParameterValue` (`self.DynamicMat`) "GlowColor" (struct :`G` 1.0 :`A` 1.0)))
    (:`2`
      (`MaterialInstanceDynamic.SetVectorParameterValue` (`self.DynamicMat`) "GlowColor" (struct :`B` 1.0 :`A` 1.0)))))

(fn `ChangesByBlockType`
  (params (CharacterRef :type "Object Object Reference") (EBlockType :type "/Game/MyBp/Block_Type Enum" :default "NewEnumerator0"))
  (locals (PlayerRef :type "Object Object Reference"))
  (set `local.PlayerRef` null CharacterRef)
  (switch `/Game/MyBp/Block_Type` EBlockType
    (:`NewEnumerator0`
      (`self.Accelerating` (`.PlayerRef` (`local.PlayerRef`))))
    (:`NewEnumerator1`
      (`self.Retarded` (`.PlayerRef` (`local.PlayerRef`))))
    (:`NewEnumerator2`
      (`self.SpawnSphere` (`.PlayerRef` (`local.PlayerRef`))))
    (:`NewEnumerator4`
      (`self.Resize` (`.PlayerRef` (`local.PlayerRef`))))))

(fn `UserConstructionScript`
  (set `self.BlockType` (cast `/Game/MyBp/Block_Type` (`KismetMathLibrary.Conv_IntToByte` (`KismetMathLibrary.RandomIntegerInRange` 0 20))))
  (if (`|EnumEquality` (`self.BlockType`) "NewEnumerator3")
    (set `self.MaxLife` 2147483647)
    (else
      (set `self.MaxLife` (`KismetMathLibrary.RandomIntegerInRange` 1 3))))
  (bind _returnvalue (`PrimitiveComponent.CreateDynamicMaterialInstance` (`self.Cube`) 0 "/Engine/VREditor/BasicMeshes/M_Floor_01.M_Floor_01" "None"))
  (set `self.DynamicMat` _returnvalue)
  (if (<= (`self.BlockType`) 4)
    (switch `/Game/MyBp/Block_Type` (`self.BlockType`)
      (:`NewEnumerator0`
        (`MaterialInstanceDynamic.SetVectorParameterValue` (`self.DynamicMat`) "FloorColor" (struct :`R` 1.0 :`G` 0.5 :`A` 1.0))
        (switch `int` (`self.MaxLife`) :!label _label
          (:`1`
            (`MaterialInstanceDynamic.SetVectorParameterValue` (`self.DynamicMat`) "GlowColor" (struct :`G` 1.0 :`A` 1.0)))
          (:`2`
            (`MaterialInstanceDynamic.SetVectorParameterValue` (`self.DynamicMat`) "GlowColor" (struct :`B` 1.0 :`A` 1.0)))
          (:`3`
            (`MaterialInstanceDynamic.SetVectorParameterValue` (`self.DynamicMat`) "GlowColor" (struct :`R` 0.5 :`B` 1.0 :`A` 1.0)))))
      (:`NewEnumerator1`
        (`MaterialInstanceDynamic.SetVectorParameterValue` (`self.DynamicMat`) "FloorColor" (struct :`R` 0.00855 :`G` 0.004286 :`B` 0.822917 :`A` 1.0))
        (goto _label))
      (:`NewEnumerator2`
        (`MaterialInstanceDynamic.SetVectorParameterValue` (`self.DynamicMat`) "FloorColor" (struct :`G` 1.0 :`A` 1.0))
        (goto _label))
      (:`NewEnumerator3`
        (`MaterialInstanceDynamic.SetVectorParameterValue` (`self.DynamicMat`) "FloorColor" (struct :`R` 1.0 :`G` 1.0 :`B` 1.0 :`A` 1.0))
        (goto _label))
      (:`NewEnumerator4`
        (`MaterialInstanceDynamic.SetVectorParameterValue` (`self.DynamicMat`) "FloorColor" (struct :`R` 0.5 :`B` 1.0 :`A` 1.0))))
    (else
      (goto _label))))