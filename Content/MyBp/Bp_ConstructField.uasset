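; Bp_ConstructField lays out a field of child actors in a grid sized by ArraySizeX and ArraySizeY.
; Its construction script runs nested loops at 200-unit spacing, scaling Y by the actor right vector's Y component and X by a zero-rotation forward vector.
; Each row also gets a child actor before the inner loop, which shares its position with that row's first inner-loop child.
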(fn `UserConstructionScript`
  (locals (Yoffset :type "Float (double-precision)"))
  (for _index (range (+ (`self.ArraySizeX`) 1))
    (set `local.Yoffset` (* (* _index 200) (`.Y` (`KismetMathLibrary.BreakVector3f` (`self.GetActorRightVector`)))))
    (`AddComponent|NODE_AddChildActorComponent-0` :`RelativeTransform` (`KismetMathLibrary.MakeTransform` (`KismetMathLibrary.MakeVector` 0.0 (`local.Yoffset`))))
    (for _index_2 (range (+ (`self.ArraySizeY`) 1))
      (`AddComponent|NODE_AddChildActorComponent-1` :`RelativeTransform` (`KismetMathLibrary.MakeTransform` (`KismetMathLibrary.MakeVector` (* (* _index_2 200) (`KismetMathLibrary.BreakVector3f` (`KismetMathLibrary.GetForwardVector` (struct)))) (`local.Yoffset`)))))))